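; BP_RiverTile is a river segment of procedurally chained terrain that spawns logs and extends the level as the player advances.
; A self-rescheduling random timer runs SpawnCar, which, despite its name, spawns BP_Log at LogSpawnPoint.
; The player's first overlap with the Box spawns a random road, grass or river tile at the Arrow.
; Random log scaling exists but is disconnected.
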(event `SpawnCar`
  (bind _returnvalue (`|SpawnActorFromClass` "/Game/BP_Log.BP_Log_C" (`SceneComponent.K2_GetComponentToWorld` (`self.LogSpawnPoint`)) "Undefined" "MultiplyWithRoot" null null))
  (`KismetSystemLibrary.K2_SetTimerDelegate` (delegate `SpawnCar`) (`KismetMathLibrary.RandomFloatInRange` 1.5 3.5)))

(event `self.ReceiveBeginPlay`
  (`KismetSystemLibrary.K2_SetTimerDelegate` (delegate `SpawnCar`) (`KismetMathLibrary.RandomFloatInRange` 1.5 3.5)))

(event `self.Box.OnComponentBeginOverlap`
  (params (OverlappedComponent :type "PrimitiveComponent Object Reference") (OtherActor :type "Actor Object Reference") (OtherComp :type "PrimitiveComponent Object Reference") (OtherBodyIndex :type Integer) (bFromSweep :type Boolean) (SweepResult :type "HitResult Structure (by ref)"))
  (bind _returnvalue (`SceneComponent.K2_GetComponentToWorld` (`self.Arrow`)))
  (cast `/Game/BP_CTR_PlayerCharacter` OtherActor)
  (`/Engine/EditorBlueprintResources/StandardMacros.DoOnce` false
    (:`Completed`
      (switch `int` (`KismetMathLibrary.RandomIntegerInRange` 0 2)
        (:`0`
          (`|SpawnActorFromClass` "/Game/BP_RoadTile.BP_RoadTile_C" _returnvalue "Undefined" "MultiplyWithRoot" null null))
        (:`1`
          (`|SpawnActorFromClass` "/Game/BP_GrassTile.BP_GrassTile_C" _returnvalue "Undefined" "MultiplyWithRoot" null null))
        (:`2`
          (`|SpawnActorFromClass` "BP_RiverTile_C" _returnvalue "Undefined" "MultiplyWithRoot" null null))))))

(fn `UserConstructionScript`)