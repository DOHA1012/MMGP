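; BP_GrassTile is a grass tile for procedurally generated terrain that carries random obstacles and spawns the next tile as the player advances.
; On BeginPlay it rolls a low chance for each evenly spaced slot along the world X axis to spawn a BP_Obstacle.
; The player character's first overlap with its Box spawns a random road, grass or river tile at the Arrow's transform, with DoOnce preventing repeats.
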(event `self.Box.OnComponentBeginOverlap`
  (params (OverlappedComponent :type "PrimitiveComponent Object Reference") (OtherActor :type "Actor Object Reference") (OtherComp :type "PrimitiveComponent Object Reference") (OtherBodyIndex :type Integer) (bFromSweep :type Boolean) (SweepResult :type "HitResult Structure (by ref)"))
  (bind _returnvalue (`SceneComponent.K2_GetComponentToWorld` (`self.Arrow`)))
  (cast `/Game/BP_CTR_PlayerCharacter` OtherActor)
  (`/Engine/EditorBlueprintResources/StandardMacros.DoOnce` false
    (:`Completed`
      (switch `int` (`KismetMathLibrary.RandomIntegerInRange` 0 2)
        (:`0`
          (`|SpawnActorFromClass` "/Game/BP_RoadTile.BP_RoadTile_C" _returnvalue "Undefined" "MultiplyWithRoot" null null))
        (:`1`
          (`|SpawnActorFromClass` "BP_GrassTile_C" _returnvalue "Undefined" "MultiplyWithRoot" null null))
        (:`2`
          (`|SpawnActorFromClass` "/Game/BP_RiverTile.BP_RiverTile_C" _returnvalue "Undefined" "MultiplyWithRoot" null null))))))

(event `self.ReceiveBeginPlay`
  (for _index (range -4 5)
    (if (< (`KismetMathLibrary.RandomFloatInRange` 0.0 1.0) 0.2)
      (`|SpawnActorFromClass` "/Game/BP_Obstacle.BP_Obstacle_C" (`KismetMathLibrary.MakeTransform` (+ (`KismetMathLibrary.MakeVector` (`KismetMathLibrary.Conv_IntToDouble` (* _index 100))) (`self.K2_GetActorLocation`))) "Undefined" "MultiplyWithRoot" null null))))

(fn `UserConstructionScript`)