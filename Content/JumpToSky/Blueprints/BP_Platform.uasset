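; BP_Platform is a Doodle Jump-style platform that bounces BP_Doodle_Character upward when it overlaps the box while falling from above.
; BeginPlay makes trap platforms breakable, otherwise randomly rolls a moving, spring or plain type, sets special materials, and may spawn a rocket pickup on plain ones.
; On landing, breakable platforms fall with physics and are destroyed, springs super-launch, and others use a DoOnce-throttled jump.
; Tick slides moving platforms along a time-offset sine on Y.
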(event `self.Box.OnComponentBeginOverlap`
  (params (OverlappedComponent :type "PrimitiveComponent Object Reference") (OtherActor :type "Actor Object Reference") (OtherComp :type "PrimitiveComponent Object Reference") (OtherBodyIndex :type Integer) (bFromSweep :type Boolean) (SweepResult :type "HitResult Structure (by ref)"))
  (bind (_returnvalue_x _returnvalue_y _returnvalue_z) (`KismetMathLibrary.BreakVector` (`self.K2_GetActorLocation`)))
  (bind _asbp_doodle_character (cast `/Game/JumpToSky/BP_Doodle_Character` OtherActor))
  (bind (_returnvalue_x_2 _returnvalue_y_2 _returnvalue_z_2) (`KismetMathLibrary.BreakVector` (`self.GetVelocity` _asbp_doodle_character)))
  (bind (_returnvalue_x_3 _returnvalue_y_3 _returnvalue_z_3) (`KismetMathLibrary.BreakVector` (`self.K2_GetActorLocation` _asbp_doodle_character)))
  (if (and (< _returnvalue_z_2 0.0) (> _returnvalue_z_3 _returnvalue_z))
    (if (`self.IsBreakable`)
      (`PrimitiveComponent.SetSimulatePhysics` (`self.StaticMesh`) true)
      (`KismetSystemLibrary.Delay` 1.0)
      (`self.K2_DestroyActor`)
      (elif (`self.IsSpring`)
        (`Character.LaunchCharacter` _asbp_doodle_character (`KismetMathLibrary.MakeVector` 0.0 0.0 (`self.SuperJumpPower`)) false true)
        (else
          (`/Engine/EditorBlueprintResources/StandardMacros.DoOnce` false :!label _label
            (:`Completed`
              (`Character.LaunchCharacter` _asbp_doodle_character (`KismetMathLibrary.MakeVector` 0.0 0.0 (`self.JumpPower`)) false true)
              (`KismetSystemLibrary.Delay` 0.2)
              (goto _label :!via `Reset`))))))))

(event `self.ReceiveBeginPlay`
  (set `self.StartLocation` (`self.K2_GetActorLocation`))
  (if (`self.IsTrap`)
    (set `self.IsBreakable` true)
    (`PrimitiveComponent.SetMaterial` (`self.StaticMesh`) 0 "/Game/JumpToSky/Blueprints/M_Platform_Brown.M_Platform_Brown")
    (else
      (set `self.IsMoving` (`KismetMathLibrary.RandomBoolWithWeight` 0.3))
      (set `self.TimeOffset` (`KismetMathLibrary.RandomFloatInRange` 0.0 10.0))
      (if (`self.IsMoving`)
        (`PrimitiveComponent.SetMaterial` (`self.StaticMesh`) 0 "/Game/JumpToSky/Blueprints/M_Water.M_Water")
        (else
          (bind _output_get (set `self.IsSpring` (`KismetMathLibrary.RandomBoolWithWeight` 0.1)))
          (if _output_get
            (`PrimitiveComponent.SetMaterial` (`self.StaticMesh`) 0 "/Game/JumpToSky/Blueprints/M_Platform_White.M_Platform_White")
            (elif (`KismetMathLibrary.RandomBoolWithWeight` 0.08)
              (`|SpawnActorFromClass` "/Game/JumpToSky/Blueprints/BP_Item_Rocket.BP_Item_Rocket_C" (`KismetMathLibrary.MakeTransform` (+ (`self.K2_GetActorLocation`) (0.0 0.0 50.0))) "Undefined" "MultiplyWithRoot" null null))))))))

(event `self.ReceiveTick`
  (params (DeltaSeconds :type "Float (single-precision)"))
  (bind (_startlocation_x _startlocation_y _startlocation_z) (`KismetMathLibrary.BreakVector` (`self.StartLocation`)))
  (if (`self.IsMoving`)
    (`self.K2_SetActorLocation` (`KismetMathLibrary.MakeVector` _startlocation_x (+ 0.0 (* (`KismetMathLibrary.Sin` (* (+ (`KismetSystemLibrary.GetGameTimeInSeconds`) (`self.TimeOffset`)) (`self.MoveSpeed`))) (`self.MoveRange`))) _startlocation_z))))

(fn `UserConstructionScript`)