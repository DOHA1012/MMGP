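; Platform manager for a vertical climbing game that spawns BP_Platform actors ever higher as the player ascends.
; It pre-spawns a batch on BeginPlay, then Tick adds more whenever the player nears the highest spawn height.
; Each platform gets a random Y offset, with an occasional trap variant offset on X near the next height.
; CalculateGap randomizes vertical spacing, widening its upper limit logarithmically with height up to a cap.
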(event `SpawnOnePlatform`
  (bind _nextspawnheight (`self.NextSpawnHeight`))
  (`|SpawnActorFromClass` "/Game/JumpToSky/Blueprints/BP_Platform.BP_Platform_C" (`KismetMathLibrary.MakeTransform` (`KismetMathLibrary.MakeVector` 0.0 (`KismetMathLibrary.RandomFloatInRange` -300.0 300.0) (`self.NextSpawnHeight`))) "Undefined" "MultiplyWithRoot" null false null)
  (set `self.NextSpawnHeight` (+ _nextspawnheight (`self.CalculateGap` _nextspawnheight)))
  (if (`KismetMathLibrary.RandomBoolWithWeight` 0.3)
    (`|SpawnActorFromClass` "/Game/JumpToSky/Blueprints/BP_Platform.BP_Platform_C" (`KismetMathLibrary.MakeTransform` (`KismetMathLibrary.MakeVector` (`KismetMathLibrary.RandomFloatInRange` -350.0 350.0) 0.0 (+ (`self.NextSpawnHeight`) (`KismetMathLibrary.RandomFloatInRange` -150.0 150.0)))) "Undefined" "MultiplyWithRoot" null true null)))

(event `self.ReceiveBeginPlay`
  (for _ (range 21)
    (`self.SpawnOnePlatform`)))

(event `self.ReceiveTick`
  (params (DeltaSeconds :type "Float (single-precision)"))
  (bind (_returnvalue_x _returnvalue_y _returnvalue_z) (`KismetMathLibrary.BreakVector` (`self.K2_GetActorLocation` (`GameplayStatics.GetPlayerCharacter` 0))))
  (if (< (- (`self.NextSpawnHeight`) _returnvalue_z) 1500.0)
    (`self.SpawnOnePlatform`)))

(fn `CalculateGap`
  (params (CurrentScore :type "Float (double-precision)"))
  (returns (FinalGap :type "Float (double-precision)"))
  (return (`KismetMathLibrary.RandomFloatInRange` (`self.MinGap`) (`KismetMathLibrary.FClamp` (+ (* (`KismetMathLibrary.Loge` (+ CurrentScore 10.0)) (`self.DifficultySpeed`)) (`self.MinGap`)) (`self.MinGap`) (`self.AbsoluteMaxGap`)))))

(fn `UserConstructionScript`)