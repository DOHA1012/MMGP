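; BP_RiverTile is a river tile for a Crossy Road-style game that spawns logs and kills the player on contact with its water.
; From BeginPlay, a self-rescheduling timer event, named SpawnCar, spawns a BP_Log at LogSpawnPoint at random intervals.
; Overlapping WaterDeathBox runs the player character's game-over process and pauses the game, guarded by a DoOnce.
; A random log-scaling node is left unconnected.
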(event `SpawnCar`
  (bind _returnvalue (`|SpawnActorFromClass` "/Game/CrossyRoad/Blueprints/Actors/BP_Log.BP_Log_C" (`SceneComponent.K2_GetComponentToWorld` (`self.LogSpawnPoint`)) "Undefined" "MultiplyWithRoot" null null))
  (`KismetSystemLibrary.K2_SetTimerDelegate` (delegate `SpawnCar`) (`KismetMathLibrary.RandomFloatInRange` 1.5 3.5)))

(event `self.ReceiveBeginPlay`
  (`KismetSystemLibrary.K2_SetTimerDelegate` (delegate `SpawnCar`) (`KismetMathLibrary.RandomFloatInRange` 1.5 3.5)))

(event `self.WaterDeathBox.OnComponentBeginOverlap`
  (params (OverlappedComponent :type "PrimitiveComponent Object Reference") (OtherActor :type "Actor Object Reference") (OtherComp :type "PrimitiveComponent Object Reference") (OtherBodyIndex :type Integer) (bFromSweep :type Boolean) (SweepResult :type "HitResult Structure (by ref)"))
  (bind _asbp_ctr_player_character (cast `/Game/CrossyRoad/Blueprints/Core/BP_CTR_PlayerCharacter` OtherActor))
  (`/Engine/EditorBlueprintResources/StandardMacros.DoOnce` false
    (:`Completed`
      (`KismetSystemLibrary.PrintString` "Hello")
      (`/Game/CrossyRoad/Blueprints/Core/BP_CTR_PlayerCharacter.GameOver_Process` _asbp_ctr_player_character)
      (`GameplayStatics.SetGamePaused` true))))

(fn `UserConstructionScript`)