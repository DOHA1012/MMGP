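; Map manager for a Crossy Road-style game that builds a randomized strip of tiles when play begins.
; BeginPlay calls SpawnOneTile in a fixed loop, and each call picks one of three spawn branches at random.
; All branches spawn at NextSpawnLocation with the same rotation, then share a step that advances that location along +Y by a constant spacing.
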(event `self.ReceiveBeginPlay`
  (for _ (range 21)
    (`self.SpawnOneTile`)))

(event `SpawnOneTile`
  (bind _nextspawnlocation (`self.NextSpawnLocation`))
  (switch `int` (`KismetMathLibrary.RandomIntegerInRange` 0 2)
    (:`0`
      (`|SpawnActorFromClass` "/Game/CrossyRoad/Blueprints/Tiles/BP_GrassTile.BP_GrassTile_C" (`KismetMathLibrary.MakeTransform` _nextspawnlocation (struct :`Yaw` 90.0)) "Undefined" "MultiplyWithRoot" null null))
    (:`1`
      (`|SpawnActorFromClass` "/Game/CrossyRoad/Blueprints/Tiles/BP_RoadTile.BP_RoadTile_C" (`KismetMathLibrary.MakeTransform` _nextspawnlocation (struct :`Yaw` 90.0)) "Undefined" "MultiplyWithRoot" null null))
    (:`2`
      (`|SpawnActorFromClass` "/Game/CrossyRoad/Blueprints/Tiles/BP_RiverTile.BP_RiverTile_C" (`KismetMathLibrary.MakeTransform` _nextspawnlocation (struct :`Yaw` 90.0)) "Undefined" "MultiplyWithRoot" null null)))
  (set `self.NextSpawnLocation` (+ (`self.NextSpawnLocation`) (0.0 100.0 0.0))))

(fn `UserConstructionScript`)