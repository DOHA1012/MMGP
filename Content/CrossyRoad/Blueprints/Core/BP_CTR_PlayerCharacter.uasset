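; Player character for the CrossyRoad minigame, handling HUD creation, timer text updates and game over.
; Tile spawn requests are forwarded to BP_MapManager.
; Both game-over events share one chain that disables input, movement and collision, submits the score to PlayFab as Score_CrossToRoad, then shows the game-over widget and pauses.
; That widget receives Score_JumpToSky as its statistic name, differing from the saved one, and both PlayFab callbacks are empty.
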(event `self.ReceiveBeginPlay`
  (bind _returnvalue (`|CreateWidget` "/Game/CrossyRoad/UI/WBP_HUD.WBP_HUD_C"))
  (`UserWidget.AddToViewport` _returnvalue 0))

(event `self.UpdateTimerUI`
  (params (CurrentTime :type "Float (single-precision)"))
  (bind _foundwidgets (`WidgetBlueprintLibrary.GetAllWidgetsOfClass` "/Game/StackToTower/WBP/WBP_Timer.WBP_Timer_C"))
  (bind _output (`|GetArrayItem` _foundwidgets))
  (`/Game/StackToTower/WBP/WBP_Timer.HidePillar` _output)
  (`TextBlock.SetText` (`/Game/StackToTower/WBP/WBP_Timer.Text_Time` _output) (`KismetTextLibrary.Conv_DoubleToText` CurrentTime "HalfToEven" false true 1 324 0 0)))

(event `self.RequestSpawnTile`
  (bind _returnvalue (`GameplayStatics.GetActorOfClass` "/Game/CrossyRoad/Blueprints/Core/BP_MapManager.BP_MapManager_C"))
  (bind _asbp_map_manager (cast `/Game/CrossyRoad/Blueprints/Core/BP_MapManager` _returnvalue))
  (`/Game/CrossyRoad/Blueprints/Core/BP_MapManager.SpawnOneTile` _asbp_map_manager))

(event `Game Over Process`
  (`self.DisableInput` null :!label _label)
  (`MovementComponent.StopMovementImmediately` (`self.CharacterMovement`))
  (`self.SetActorEnableCollision` false)
  (bind _returnvalue (`|GenericCreateObject` "/Script/PlayFab.PlayFabJsonObject"))
  (`PlayFabJsonObject.SetStringField` _returnvalue "StatisticName" "Score_CrossToRoad")
  (`PlayFabJsonObject.SetNumberField` _returnvalue "Value" (`KismetMathLibrary.Conv_IntToDouble` (`KismetMathLibrary.FTrunc` (`KismetMathLibrary.Conv_IntToDouble` (`self.CurrentScore`)))))
  (`PlayFabClientAPI.UpdatePlayerStatistics` (make `ClientUpdatePlayerStatisticsRequest` null (`|MakeArray` _returnvalue)) (delegate `저장성공`) (delegate `저장실패`)
    (:`then`
      (bind _returnvalue_2 (`|CreateWidget` "/Game/JumpToSky/WBP_GameOver2.WBP_GameOver2_C" null "Score_JumpToSky"))
      (`UserWidget.AddToViewport` _returnvalue_2 0)
      (set `PlayerController.bShowMouseCursor` true (`GameplayStatics.GetPlayerController` 0))
      (`GameplayStatics.SetGamePaused` true))))

(event `self.StartGameOverSequence`
  (goto _label))

(event `저장성공`
  (params (result :type "ClientUpdatePlayerStatisticsResult Structure") (customData :type "Object Object Reference")))

(event `저장실패`
  (params (error :type "PlayFabError Structure") (customData :type "Object Object Reference")))

(fn `UserConstructionScript`)