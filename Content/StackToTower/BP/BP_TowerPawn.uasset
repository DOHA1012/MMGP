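; Player pawn for a timed block-stacking tower game; a one-second countdown triggers the paused game-over screen.
; Spawns random blocks above the tower: A/D shift, Q/E rotate the same way, Space speeds descent.
; A swept-move hit or the block's Landed dispatcher enables physics and spawns the next block.
; Tick derives CurrentScore from block heights, which drives spawn height and smoothly raises BP_GameCamera.
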(event `TriggerGameOver`
  (bind _returnvalue (`|CreateWidget` "/Game/StackToTower/WBP/WBP_GameOver.WBP_GameOver_C"))
  (`UserWidget.AddToViewport` _returnvalue 0)
  (set `PlayerController.bShowMouseCursor` true (`GameplayStatics.GetPlayerController` 0))
  (`GameplayStatics.SetGamePaused` true))

(event `self.ReceiveBeginPlay`
  (bind _outactors (`GameplayStatics.GetAllActorsOfClass` "/Game/StackToTower/BP/BP_GameCamera.BP_GameCamera_C"))
  (set `self.MyCamera` (`|GetArrayItem` _outactors))
  (bind _returnvalue (`|CreateWidget` "/Game/StackToTower/WBP/WBP_Timer.WBP_Timer_C"))
  (`UserWidget.AddToViewport` _returnvalue 0)
  (`KismetSystemLibrary.K2_SetTimerDelegate` (delegate `DecreaseTime`) 1.0 true)
  (`self.SpawnNewBlock`)
  (set `self.NextBlockIndex` (`KismetMathLibrary.RandomIntegerInRange` 0 6))
  (set `self.DefaultZ` (.z (`self.K2_GetActorLocation` (`self.MyCamera`)))))

(event `DecreaseTime`
  (bind _output_get (set `self.TimeLeft` (- (`self.TimeLeft`) 1.0)))
  (if (<= _output_get 0.0)
    (`self.TriggerGameOver`)))

(event `SpawnNewBlock`
  (bind _blocklist (`self.BlockList`))
  (bind _returnvalue (`|SpawnActorFromClass` (`|GetArrayItem` _blocklist (`self.NextBlockIndex`)) (`KismetMathLibrary.MakeTransform` (`KismetMathLibrary.MakeVector` 0.0 0.0 (+ (`self.CurrentScore`) 1500.0)) (struct :`Pitch` 90.0 :`Roll` 90.0)) "AlwaysSpawn" "MultiplyWithRoot" null null))
  (bind _output_get (set `self.HoldingBlock` _returnvalue))
  (set `self.NextBlockIndex` (`KismetMathLibrary.RandomIntegerInRange` 0 (`KismetArrayLibrary.Array_LastIndex` _blocklist)))
  (bind _asbp_block_i (cast `/Game/StackToTower/Block/BP/BP_Block_I` _output_get))
  (add `/Game/StackToTower/Block/BP/BP_Block_I.Dispatch_Landed` _asbp_block_i (delegate `Dispatch_Landed_이벤트`)))

(event `Dispatch_Landed_이벤트`
  (bind _cube (`/Game/StackToTower/Block/BP/BP_Block_I.Cube` (`self.HoldingBlock`)))
  (`PrimitiveComponent.SetSimulatePhysics` _cube true)
  (`PrimitiveComponent.SetLinearDamping` _cube 1.5)
  (set `self.HoldingBlock` null)
  (`self.SpawnNewBlock`))

(event `Key|A`
  (params (Key :type "Key Structure"))
  (bind _holdingblock (`self.HoldingBlock`))
  (:`Pressed`
    (`/Engine/EditorBlueprintResources/StandardMacros.IsValid` _holdingblock
      (:`Is Valid`
        (`self.K2_AddActorWorldOffset` _holdingblock (50.0 0.0 0.0) false false)))))

(event `Key|D`
  (params (Key :type "Key Structure"))
  (bind _holdingblock (`self.HoldingBlock`))
  (:`Pressed`
    (`/Engine/EditorBlueprintResources/StandardMacros.IsValid` _holdingblock
      (:`Is Valid`
        (`self.K2_AddActorWorldOffset` _holdingblock (-50.0 0.0 0.0) false false)))))

(event `Key|SpaceBar`
  (params (Key :type "Key Structure"))
  (:`Pressed`
    (set `self.DropSpeed` -50.0))
  (:`Released`
    (set `self.DropSpeed` -2.0)))

(event `self.ReceiveTick`
  (params (DeltaSeconds :type "Float (single-precision)"))
  (bind _holdingblock (`self.HoldingBlock`))
  (bind _mycamera (`self.MyCamera`))
  (bind (_returnvalue_x _returnvalue_y _returnvalue_z) (`KismetMathLibrary.BreakVector` (`self.K2_GetActorLocation` _mycamera)))
  (`self.CalculateHeight`)
  (`self.K2_SetActorLocation` _mycamera (`KismetMathLibrary.MakeVector` _returnvalue_x _returnvalue_y (`KismetMathLibrary.FInterpTo` _returnvalue_z (+ (`self.DefaultZ`) (`self.CurrentScore`)) DeltaSeconds 2.0)) false false)
  (set `self.CurrentScore` 0.0)
  (bind _outactors (`GameplayStatics.GetAllActorsOfClass` "/Game/StackToTower/Block/BP/BP_Block_I.BP_Block_I_C"))
  (for _array_element _outactors
    (bind _asbp_block_i (cast `/Game/StackToTower/Block/BP/BP_Block_I` _array_element))
    (if (`SceneComponent.IsSimulatingPhysics` (`/Game/StackToTower/Block/BP/BP_Block_I.Cube` _asbp_block_i) "None")
      (bind (_returnvalue_x_2 _returnvalue_y_2 _returnvalue_z_2) (`KismetMathLibrary.BreakVector` (`self.K2_GetActorLocation` _array_element)))
      (set `self.CurrentScore` (- (`KismetMathLibrary.FMax` _returnvalue_z_2 (`self.CurrentScore`)) 100.0))))
  (`self.K2_SetActorLocation` (`KismetMathLibrary.MakeVector` _returnvalue_x_2 _returnvalue_y_2 (`KismetMathLibrary.FInterpTo` _returnvalue_z_2 (+ (`self.CurrentScore`) (`self.DefaultZ`)) (`GameplayStatics.GetWorldDeltaSeconds`) 1.0)))
  (`/Engine/EditorBlueprintResources/StandardMacros.IsValid` _holdingblock
    (:`Is Valid`
      (bind _sweephitresult (`self.K2_AddActorWorldOffset` _holdingblock (`KismetMathLibrary.MakeVector` 0.0 0.0 (`self.DropSpeed`)) true false))
      (if (`GameplayStatics.BreakHitResult` _sweephitresult)
        (`self.K2_AddActorWorldOffset` _holdingblock (`KismetMathLibrary.MakeVector` 0.0 0.0 (`self.DropSpeed`)) true false)
        (`KismetSystemLibrary.PrintString` (`KismetSystemLibrary.GetDisplayName` null))
        (`PrimitiveComponent.SetSimulatePhysics` (`/Game/StackToTower/Block/BP/BP_Block_I.Cube` _holdingblock) true)
        (set `self.HoldingBlock` null)
        (`KismetSystemLibrary.Delay` 2.0)
        (`self.SpawnNewBlock`)))))

(event `Key|Q`
  (params (Key :type "Key Structure"))
  (:`Pressed`
    (`/Engine/EditorBlueprintResources/StandardMacros.IsValid` (`self.HoldingBlock`)
      (:`Is Valid`
        (`self.K2_AddActorWorldRotation` (`self.HoldingBlock`) (struct :`Pitch` 90.0) false false :!label _label)))))

(event `Key|E`
  (params (Key :type "Key Structure"))
  (:`Pressed`
    (`/Engine/EditorBlueprintResources/StandardMacros.IsValid` (`self.HoldingBlock`)
      (:`Is Valid`
        (goto _label)))))

(fn `CalculateHeight`
  (bind _outactors (`GameplayStatics.GetAllActorsOfClass` "/Game/StackToTower/Block/BP/BP_Block_I.BP_Block_I_C"))
  (for _array_element _outactors
    (if (!= _array_element (`self.HoldingBlock`))
      (set `self.CurrentScore` (`KismetMathLibrary.FMax` (.z (`self.K2_GetActorLocation` _array_element)) (`self.CurrentScore`))))))

(fn `UserConstructionScript`)